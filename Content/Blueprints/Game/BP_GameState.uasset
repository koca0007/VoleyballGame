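; Game state Blueprint that keeps the scores of two teams as throws are won or lost.
; Two events increment Team1Score or Team2Score on the authority only.
; When Team 2 is present and Team 1 throws, a win scores for Team 1 and a loss for Team 2.
; In every other case, a win scores for Team 2 and a loss for Team 1.
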(event `AddScoreOnLoss`
  (params (IsTeam2Present :type Boolean) (IsThrowerTeam1 :type Boolean))
  (`/Engine/EditorBlueprintResources/ActorMacros.Switch Has Authority`
    (:`Authority`
      (if (and IsTeam2Present IsThrowerTeam1)
        (`/Engine/EditorBlueprintResources/StandardMacros.IncrementInt` (`self.Team2Score`))
        (else
          (`/Engine/EditorBlueprintResources/StandardMacros.IncrementInt` (`self.Team1Score`)))))))

(event `AddScoreOnWin`
  (params (IsTeam2Present :type Boolean) (IsThrowerTeam1 :type Boolean))
  (`/Engine/EditorBlueprintResources/ActorMacros.Switch Has Authority`
    (:`Authority`
      (if (and IsTeam2Present IsThrowerTeam1)
        (`/Engine/EditorBlueprintResources/StandardMacros.IncrementInt` (`self.Team1Score`))
        (else
          (`/Engine/EditorBlueprintResources/StandardMacros.IncrementInt` (`self.Team2Score`)))))))

(fn `UserConstructionScript`)