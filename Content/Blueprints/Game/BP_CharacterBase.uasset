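; Base player character for a ball game (apparently volleyball-style) with serve, throw, pass and dunk actions, plus level-dependent HUD creation and a VSync console toggle.
; A collision overlap caches the nearby BP_Ball and enables hits, which compute a velocity and launch it through server events with a multicast sound.
; Holding Serve loops a projectile-path prediction to place a landing decal; release spawns and launches a new ball on the server, unless cancelled.
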(event `self.ReceiveBeginPlay`
  (bind _returnvalue (`GameplayStatics.GetCurrentLevelName` true))
  (if (`KismetStringLibrary.NotEqual_StrStr` _returnvalue "PracticeArea")
    (bind _returnvalue_2 (`|CreateWidget` "/Game/Blueprints/UI/WBP_UI.WBP_UI_C"))
    (`UserWidget.AddToViewport` _returnvalue_2 0)
    (else
      (bind _returnvalue_3 (`|CreateWidget` "/Game/Blueprints/UI/WBP_Crosshair.WBP_Crosshair_C"))
      (`UserWidget.AddToViewport` _returnvalue_3 0))))

(event `InputAction|ToggleVSync`
  (params (Key :type "Key Structure"))
  (:`Pressed`
    (if (`self.bVsyncOn`)
      (`KismetSystemLibrary.ExecuteConsoleCommand` "r.VSync 1" null)
      (else
        (`KismetSystemLibrary.ExecuteConsoleCommand` "r.VSync 0" null)))))

(event `Server_ServeBall`
  (params (StartPoint :type "Vector Structure") (`Launch Velocity` :type "Vector Structure"))
  (bind _returnvalue (`|SpawnActorFromClass` "/Game/Blueprints/BP_Ball.BP_Ball_C" (`KismetMathLibrary.MakeTransform` StartPoint) "AlwaysSpawn" "OverrideRootScale" null null))
  (`/Game/Blueprints/BP_Ball.Throw` _returnvalue `Launch Velocity` self)
  (`self.Multicast_PlaySound`))

(event `InputAction|Serve`
  (params (Key :type "Key Structure"))
  (bind _hitdecal (`self.HitDecal`))
  (:`Pressed`
    (if (`self.IsLocallyControlled`)
      (if (`self.bReadyToServe`)
        (set `self.bServing` true)
        (set `self.bCanceled` false)
        (if (`self.bServing`) :!label _label
          (bind _output_get (set `self.ServeVelocity` (* (`KismetMathLibrary.GetForwardVector` (`self.GetControlRotation`)) (`self.ThrowStrength`))))
          (bind (_outhit _outpathpositions _outlasttracedestination) (`GameplayStatics.Blueprint_PredictProjectilePath_ByTraceChannel` (`SceneComponent.K2_GetComponentLocation` (`self.ServeLocation`)) _output_get true 0.0 "ECC_WorldStatic" false (`|MakeArray` self :!type "Actor Object Reference") "None" 0.1))
          (`SceneComponent.K2_SetWorldLocation` _hitdecal _outlasttracedestination false false)
          (`SceneComponent.SetVisibility` _hitdecal true false)
          (for _ _outpathpositions
            _)
          (`KismetSystemLibrary.Delay` (`GameplayStatics.GetWorldDeltaSeconds`))
          (goto _label))
        (else
          (`KismetSystemLibrary.PrintString` "Not ready to serve")))))
  (:`Released`
    (if (`self.bServing`)
      (if (not (`self.bCanceled`))
        (set `self.bServing` false)
        (`SceneComponent.SetVisibility` (`self.HitDecal`) false false)
        (`self.Server_ServeBall` (`SceneComponent.K2_GetComponentLocation` (`self.ServeLocation`)) (`self.ServeVelocity`))
        (set `self.bReadyToServe` false)))))

(event `InputAction|Cancel`
  (params (Key :type "Key Structure"))
  (:`Pressed`
    (if (`self.bServing`)
      (set `self.bCanceled` true)
      (set `self.bServing` false)
      (`SceneComponent.SetVisibility` (`self.HitDecal`) false false))))

(event `InputAction|Throw`
  (params (Key :type "Key Structure"))
  (:`Pressed`
    (set `self.bThrowing` true)
    (if (and (`self.bThrowing`) (`self.bCanThrow`))
      (bind _output_get (set `self.ServeVelocity` (* (`KismetMathLibrary.GetForwardVector` (`self.GetControlRotation`)) (`self.ThrowStrength`))))
      (`GameplayStatics.Blueprint_PredictProjectilePath_ByTraceChannel` (`SceneComponent.K2_GetComponentLocation` (`self.ServeLocation`)) _output_get true 0.0 "ECC_WorldStatic" false (`|MakeArray` self :!type "Actor Object Reference") "None" 0.1)))
  (:`Released`
    (if (`self.bCanThrow`)
      (set `self.bThrowing` false)
      (`SceneComponent.SetVisibility` (`self.HitDecal`) false false)
      (`self.Server_ThrowBall` (`self.ServeVelocity`)))))

(event `Server_ThrowBall`
  (params (Velocity :type "Vector Structure"))
  (if (`self.bCanThrow`)
    (`/Game/Blueprints/BP_Ball.Throw` (`self.Ball`) Velocity self)
    (`self.Multicast_PlaySound`)))

(event `self.ReceiveTick`
  (params (DeltaSeconds :type "Float (single-precision)")))

(event `InputAction|Dunk`
  (params (Key :type "Key Structure"))
  (:`Pressed`
    (if (and (not (`self.bDunking`)) (`self.bCanThrow`))
      (set `self.DunkVelocity` (* (`KismetMathLibrary.GetForwardVector` (`self.GetControlRotation`)) (`self.DunkStrength`)))
      (set `self.bDunking` true)
      (if (`self.bDunking`)
        (`self.Server_Dunk` (`self.DunkVelocity`)))))
  (:`Released`
    (set `self.bDunking` false)))

(event `Server_Dunk`
  (params (Velocity :type "Vector Structure"))
  (if (`self.bCanThrow`)
    (`/Game/Blueprints/BP_Ball.Throw` (`self.Ball`) Velocity self)
    (`self.Multicast_PlaySound`)))

(event `InputAction|Pass`
  (params (Key :type "Key Structure"))
  (:`Pressed`
    (if (and (`self.bCanThrow`) (not (`self.bPassing`)))
      (set `self.PassVelocity` (* (0.0 0.0 1.0) (`self.PassStrength`)))
      (set `self.bPassing` true)
      (if (`self.bPassing`)
        (`self.Server_Pass` (`self.PassVelocity`)))))
  (:`Released`
    (set `self.bPassing` false)))

(event `Server_Pass`
  (params (Velocity :type "Vector Structure"))
  (if (`self.bCanThrow`)
    (`/Game/Blueprints/BP_Ball.Throw` (`self.Ball`) Velocity self)
    (`self.Multicast_PlaySound`)))

(event `self.Collision.OnComponentBeginOverlap`
  (params (OverlappedComponent :type "PrimitiveComponent Object Reference") (OtherActor :type "Actor Object Reference") (OtherComp :type "PrimitiveComponent Object Reference") (OtherBodyIndex :type Integer) (bFromSweep :type Boolean) (SweepResult :type "HitResult Structure (by ref)"))
  (if (`self.ActorHasTag` OtherActor "Ball")
    (bind _asbp_ball (cast `/Game/Blueprints/BP_Ball` OtherActor))
    (set `self.Ball` _asbp_ball)
    (set `self.bCanThrow` true)))

(event `self.Collision.OnComponentEndOverlap`
  (params (OverlappedComponent :type "PrimitiveComponent Object Reference") (OtherActor :type "Actor Object Reference") (OtherComp :type "PrimitiveComponent Object Reference") (OtherBodyIndex :type Integer))
  (if (== OtherActor (`self.Ball`))
    (set `self.bCanThrow` false)))

(event `Multicast_PlaySound`
  (`GameplayStatics.PlaySoundAtLocation` "/Game/Cue_He.Cue_He" (`self.K2_GetActorLocation`) (struct) 1.0 1.0 0.0 null null null))

(event `Multicast_ReplicateCharacterRotation`)

(fn `UserConstructionScript`)